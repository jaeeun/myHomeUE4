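; Dishwasher actor that opens on BeginPlay and collects objects placed inside it.
; Two timelines slide the bottom and middle racks out and swing the door down, with CloseDoor playing both in reverse.
; Box overlaps, excluding "AMMR"-named actors, are gathered; after a retriggerable delay, static mesh actors stop simulating physics and attach to the bottom rack.
; Holding four objects starts a short timer to a delegate event.
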(event `self.ReceiveBeginPlay`
  (set `self.TopLocation` (`SceneComponent.RelativeLocation` (`self.SM_dish_washer_01_bottom`)))
  (set `self.MidLocation` (`SceneComponent.RelativeLocation` (`self.SM_dish_washer_01_mid`)))
  (`self.Open`))

(event `Open`
  (set `self.IsWorking` true)
  (`|ExecutionSequence`
    (:`then_0`
      (bind (_direction _value) (`Timeline|타임라인_0` :!via `PlayFromStart` :!label _label)
        (:`Update`
          (`|ExecutionSequence`
            (:`then_1`
              (`SceneComponent.K2_SetRelativeLocation` (`self.SM_dish_washer_01_bottom`) (+ (`self.TopLocation`) (`KismetMathLibrary.MakeVector` 0.0 (* _value 50.0))) false false))
            (:`then_2`
              (`SceneComponent.K2_SetRelativeLocation` (`self.SM_dish_washer_01_mid`) (+ (`self.MidLocation`) (`KismetMathLibrary.MakeVector` 0.0 (* _value 10.0))) false false))))
        (:`Finished`
          (set `self.IsWorking` false))))
    (:`then_1`
      (bind (_direction_2 _value_2) (`Timeline|타임라인_1` :!via `PlayFromStart` :!label _label_2)
        (:`Update`
          (`SceneComponent.K2_SetRelativeRotation` (`self.SM_dish_washer_01_door`) (`KismetMathLibrary.MakeRotator` (* _value_2 90.0)) false false))))))

(event `CloseDoor`
  (set `self.IsWorking` true)
  (`|ExecutionSequence`
    (:`then_0`
      (goto _label :!via `ReverseFromEnd`))
    (:`then_1`
      (goto _label_2 :!via `ReverseFromEnd`))))

(event `self.Box.OnComponentBeginOverlap`
  (params (OverlappedComponent :type "PrimitiveComponent Object Reference") (OtherActor :type "Actor Object Reference") (OtherComp :type "PrimitiveComponent Object Reference") (OtherBodyIndex :type Integer) (bFromSweep :type Boolean) (SweepResult :type "HitResult Structure (by ref)"))
  (if (not (`KismetStringLibrary.Contains` (`KismetSystemLibrary.GetObjectName` OtherActor) "AMMR"))
    (`KismetArrayLibrary.Array_AddUnique` (`self.Objects`) OtherActor)
    (`KismetSystemLibrary.RetriggerableDelay` 5.0)
    (for _array_element (`self.Objects`)
      (bind _asstatic_mesh_actor (cast `StaticMeshActor` _array_element))
      (`PrimitiveComponent.SetSimulatePhysics` (`StaticMeshActor.StaticMeshComponent` _asstatic_mesh_actor) false)
      (`self.K2_AttachToComponent` _asstatic_mesh_actor (`self.SM_dish_washer_01_bottom`) "None" "KeepWorld" "KeepWorld" "KeepWorld" true)
      (if (== 4 (`KismetArrayLibrary.Array_Length` (`self.Objects`)))
        (`KismetSystemLibrary.K2_SetTimerDelegate` (`|CreateDelegate` :!event `CloseDoor`) 0.5)))))

(fn `UserConstructionScript`)